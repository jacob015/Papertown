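; Knight1 is an AI-moved knight pawn that chases the player when its Move event is triggered.
; Each Tick it turns to the yaw pointing from the player toward itself, billboard-style, and hands Move to TestCharacter through AssignMoveToCharacter.
; Move runs AIMoveTo toward the player pawn, calling itself again on failure and printing a debug string on success.
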(event `self.ReceiveBeginPlay`)

(event `self.ReceiveTick`
  (params (DeltaSeconds :type "Float (single-precision)"))
  (bind (_returnvalue_roll _returnvalue_pitch _returnvalue_yaw) (`KismetMathLibrary.BreakRotator` (`KismetMathLibrary.FindLookAtRotation` (`self.K2_GetActorLocation` (`GameplayStatics.GetPlayerCharacter` 0)) (`self.K2_GetActorLocation`))))
  (`self.K2_SetActorRotation` (`KismetMathLibrary.MakeRotator` 0.0 0.0 _returnvalue_yaw))
  (bind _astest_character (cast `/Game/PapertownProject/Blueprints/Test/TestCharacter` (`GameplayStatics.GetPlayerCharacter` 0)))
  (add `/Game/PapertownProject/Blueprints/Test/TestCharacter.MoveToCharacter` _astest_character (delegate `Move`)))

(event `Move`
  (`|AIMoveTo` self (0.0 0.0 0.0) (`GameplayStatics.GetPlayerPawn` 0)
    (:`OnSuccess`
      (`KismetSystemLibrary.PrintString` "Hello"))
    (:`OnFail`
      (`self.Move`))))

(fn `UserConstructionScript`)