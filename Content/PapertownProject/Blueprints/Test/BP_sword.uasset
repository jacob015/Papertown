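; VR sword that a motion controller can pick up and drop, and that slices procedural meshes on contact.
; Pickup snaps it to the given component at a fixed grip offset with physics off; drop detaches it and restores physics.
; Blade overlap cuts along the mesh's up-vector plane, creating a capped, physics-simulated other half.
; A DoOnce, reset on end overlap, limits repeat cuts.
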(event `/Game/PapertownProject/Blueprints/VR/PickupActorInterface.Pickup`
  (params (AttachTo :type "SceneComponent Object Reference"))
  (`PrimitiveComponent.SetSimulatePhysics` (`self.StaticMeshComponent`) false)
  (`SceneComponent.K2_AttachToComponent` (`self.K2_GetRootComponent`) AttachTo "None" "SnapToTarget" "SnapToTarget" "KeepWorld" false)
  (`SceneComponent.K2_SetRelativeLocationAndRotation` (`self.StaticMeshComponent`) (1.614295 -7.088272 41.627159) (struct :`Pitch` -5.939135 :`Yaw` 0.681895 :`Roll` -98.946785) false false))

(event `/Game/PapertownProject/Blueprints/VR/PickupActorInterface.Drop`
  (`PrimitiveComponent.SetSimulatePhysics` (`self.StaticMeshComponent`) true)
  (`self.K2_DetachFromActor` "KeepWorld" "KeepWorld" "KeepWorld"))

(event `self.StaticMesh.OnComponentBeginOverlap`
  (params (OverlappedComponent :type "PrimitiveComponent Object Reference") (OtherActor :type "Actor Object Reference") (OtherComp :type "PrimitiveComponent Object Reference") (OtherBodyIndex :type Integer) (bFromSweep :type Boolean) (SweepResult :type "HitResult Structure (by ref)"))
  (bind _staticmesh (`self.StaticMesh`))
  (`/Engine/EditorBlueprintResources/StandardMacros.DoOnce` false :!label _label
    (:`Completed`
      (bind _asprocedural_mesh_component (cast `ProceduralMeshComponent` OtherComp))
      (bind _outotherhalfprocmesh (`KismetProceduralMeshLibrary.SliceProceduralMesh` _asprocedural_mesh_component (`SceneComponent.K2_GetComponentLocation` _staticmesh) (`SceneComponent.GetUpVector` _staticmesh) true "CreateNewSectionForCap" "/Game/FirstPerson/Meshes/BaseMaterial.BaseMaterial"))
      (`PrimitiveComponent.SetSimulatePhysics` _outotherhalfprocmesh true))))

(event `self.StaticMesh.OnComponentEndOverlap`
  (params (OverlappedComponent :type "PrimitiveComponent Object Reference") (OtherActor :type "Actor Object Reference") (OtherComp :type "PrimitiveComponent Object Reference") (OtherBodyIndex :type Integer))
  (goto _label :!via `Reset`))

(fn `UserConstructionScript`)