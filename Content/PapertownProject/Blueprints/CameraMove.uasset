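; CameraMove is an actor that orbits a target actor from a fixed height above it while always facing it.
; While IsStart is false, Tick accumulates an angle from RotationSpeed and the Clockwise direction.
; RotateActorAroundPoint adds StartingAngle, rotates a Radius offset around Z from the target's current location, then applies a look-at rotation.
; Without a valid target, the actor stays still.
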(event `self.ReceiveBeginPlay`
  (set `self.InitialLocation` (`self.K2_GetActorLocation`)))

(event `self.ReceiveTick`
  (params (DeltaSeconds :type "Float (single-precision)"))
  (if (not (`self.IsStart`))
    (set `self.CurrentRotation` (+ (`self.CurrentRotation`) (* (* DeltaSeconds (`self.RotationSpeed`)) (`KismetMathLibrary.SelectFloat` 1.0 -1.0 (`self.Clockwise`)))))
    (`self.RotateActorAroundPoint` self (`self.TargetActor`) (`self.InitialLocation`) (`self.Radius`) (`self.StartingAngle`) (`self.CurrentRotation`))))

(fn `RotateActorAroundPoint`
  (params (ActorToRotate :type "Actor Object Reference") (TargetActor :type "Actor Object Reference") (TargetLocation :type "Vector Structure") (Radius :type "Float (double-precision)") (Angle :type "Float (double-precision)") (`Rotation Rate` :type "Float (double-precision)"))
  (locals (LActorToRotate :type "Actor Object Reference") (LTargetActor :type "Actor Object Reference") (LLocation :type "Vector Structure") (LRadius :type "Float (double-precision)") (LAngle :type "Float (double-precision)") (LRotationRate :type "Float (double-precision)"))
  (bind _ltargetactor (`local.LTargetActor`))
  (set `local.LActorToRotate` ActorToRotate)
  (set `local.LTargetActor` TargetActor)
  (set `local.LLocation` TargetLocation)
  (set `local.LRadius` Radius)
  (set `local.LAngle` Angle)
  (set `local.LRotationRate` `Rotation Rate`)
  (`/Engine/EditorBlueprintResources/StandardMacros.IsValid` _ltargetactor
    (:`Is Valid`
      (set `local.LLocation` (`self.K2_GetActorLocation` _ltargetactor))
      (`self.K2_SetActorLocation` (`local.LActorToRotate`) (+ (+ (`local.LLocation`) (`KismetMathLibrary.RotateAngleAxis` (`KismetMathLibrary.MakeVector` (`local.LRadius`)) (+ (`local.LRotationRate`) (`local.LAngle`)) (0.0 0.0 1.0))) (0.0 0.0 2000.0)) false false)
      (`self.K2_SetActorRotation` (`KismetMathLibrary.FindLookAtRotation` (`self.K2_GetActorLocation`) (`self.K2_GetActorLocation` (`local.LTargetActor`)))))))

(fn `UserConstructionScript`)